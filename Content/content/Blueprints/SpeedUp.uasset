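; SpeedUp is an overlap-triggered actor, apparently a pickup, that recycles itself when touched.
; After the parent overlap handler runs, it checks the other actor's name for a player collision and prints a Finnish "money found" debug message on a match.
; Otherwise it calls CheckRespawnHit, but the following branch is fixed to true.
; Both paths therefore reset position and scale, then feed the scale result into ResetValue.
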(event EventBeginPlay
  (|CallParentFunction) ; This node is disabled and will not be called.\nDrag off pins to build functionality.
)

(event Collision|EventActorBeginOverlap
  (params (OtherActor :type Actor%20Object%20Reference))
  (bind _returnvalue (Utilities|GetObjectName OtherActor))
  (|CallParentFunction OtherActor)
  (bind _playercollision (CallFunction|CheckPlayerCollision _returnvalue))
  (if _playercollision
    (Development|PrintString "Raha L;ytyi")
    (CallFunction|ResetPosition :!label _label)
    (bind _scale (CallFunction|ResetScale))
    (CallFunction|ResetValue _scale)
    (else
      (CallFunction|CheckRespawnHit _returnvalue)
      (if true
        (goto _label)))))

(event EventTick
  (params (DeltaSeconds :type Float%20%28single-precision%29))
  (|CallParentFunction DeltaSeconds) ; This node is disabled and will not be called.\nDrag off pins to build functionality.
)

(fn ConstructionScript
  (|CallParentFunction))