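; Projectile actor with helper functions for hit checks and for resetting itself with randomized size and height.
; Collision checks compare object names against player character 0 and a stored destroy-trigger name.
; The resets apply a random uniform scale, returning the value before its division, and restore the initial X/Y with a random Z.
; The event graph is empty, so nothing in this Blueprint calls these functions or drives movement.
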(event EventBeginPlay)

(event Collision|EventActorBeginOverlap
  (params (OtherActor :type Actor%20Object%20Reference)))

(event EventTick
  (params (DeltaSeconds :type Float%20%28single-precision%29)))

(fn ConstructionScript)

(fn CheckPlayerCollision
  (params (OtherObjectname :type String))
  (return (Utilities|Enum|Equal(Enum) OtherObjectname (Utilities|GetObjectName (Game|GetPlayerCharacter 0)))))

(fn CheckRespawnHit
  (params (CheckObjectName :type String))
  (return (Utilities|Enum|Equal(Enum) CheckObjectName (Variables|Default|GetDestroyTriggerName))))

(fn ResetScale
  (bind _output_get (Variables|Default|SetScale (Math|Random|RandomFloatinRange 2.5 4.0)))
  (Transformation|SetActorScale3D (Math|Vector|MakeVector (/ _output_get 5.0) (/ _output_get 5.0) (/ _output_get 5.0)))
  (return _output_get))

(fn ResetPosition
  (bind _initialposition (Variables|Default|GetInitialPosition))
  (bind (_x _y) (Math|Vector|BreakVector _initialposition))
  (Transformation|SetActorLocation (Math|Vector|MakeVector _x _y (Math|Random|RandomFloatinRange 1.3e+02 1.4e+02)) false false))