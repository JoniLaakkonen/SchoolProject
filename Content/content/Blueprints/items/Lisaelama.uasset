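; Lisaelama is a heart pickup item, built on a parent Blueprint that supplies the collision checks and reset functions.
; On player overlap it calls the heart-collected dispatcher with 1 and plays a persistent eat sound, stored on the game instance, with a sound mix.
; Instead of being destroyed, it resets position and scale, and does the same after the respawn-trigger check on other overlaps.
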(event EventBeginPlay
  (|CallParentFunction) ; This node is disabled and will not be called.\nDrag off pins to build functionality.
)

(event Collision|EventActorBeginOverlap
  (params (OtherActor :type Actor%20Object%20Reference))
  (bind _returnvalue (Utilities|GetObjectName OtherActor))
  ;[1 1 1] Check if hearth hit...
  (|CallParentFunction OtherActor)
  ;[1 1 1] ... player
  (bind _playercollision (CallFunction|CheckPlayerCollision _returnvalue))
  (if _playercollision
    (Default|CallHeartCollectedED 1)
    (CallFunction|Spawneatsound)
    ;[1 1 1] ... fake moneybag destroy and reset
    (CallFunction|ResetPosition :!label _label)
    (CallFunction|ResetScale)
    (else
      ;[1 1 1] ... Respawn trigger
      (CallFunction|CheckRespawnHit _returnvalue)
      (if true
        (goto _label)))))

(event EventTick
  (params (DeltaSeconds :type Float%20%28single-precision%29))
  (|CallParentFunction DeltaSeconds) ; This node is disabled and will not be called.\nDrag off pins to build functionality.
)

(fn ConstructionScript
  (|CallParentFunction))

(fn Spawneatsound
  ;[1 1 1] spawn sound
  (bind _returnvalue (Audio|SpawnSound2D "/Game/content/Sounds/eat.eat" 1.0 1.0 0.0 0 true))
  (bind _asitempickp (Utilities|Casting|CastToItempickp (Game|GetGameInstance)))
  (Variables|/Game/content/Blueprints/Itempickp.Itempickp_C|SetItempickup _asitempickp _returnvalue)
  (Class|GameplayStatics|SetBaseSoundMix "/Game/content/Sounds/MyEffectSoundmix.MyEffectSoundmix"))