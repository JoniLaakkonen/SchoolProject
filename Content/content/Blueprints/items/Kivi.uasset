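; Kivi is a rock projectile actor that moves every tick by its speed scaled by global time dilation.
; On overlap with the player it signals the rock hit and plays a 2D explosion sound.
; It then fakes destruction by resetting position and scale and toggling a move permission around a random delay, so the actor is reused.
; Non-player overlaps go through a respawn-trigger check and join the same reset path.
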(event EventBeginPlay
  (|CallParentFunction) ; This node is disabled and will not be called.\nDrag off pins to build functionality.
)

(event Collision|EventActorBeginOverlap
  (params (OtherActor :type Actor%20Object%20Reference))
  (bind _returnvalue (Utilities|GetObjectName OtherActor))
  ;[1 1 1] Check if projectile hit...
  (|CallParentFunction OtherActor)
  ;[1 1 1] ... player
  (bind _playercollision (CallFunction|CheckPlayerCollision _returnvalue))
  (if _playercollision
    (Default|CallIgotHitbyRock (Variables|Default|GetHit))
    (CallFunction|Spawnkivisound)
    ;[1 1 1] ... fake projectile destroy and reset
    (CallFunction|ResetPosition :!label _label)
    (CallFunction|ResetScale)
    (Variables|Default|Setpermit%20to%20move false)
    (Utilities|FlowControl|Delay (Math|Random|RandomFloatinRange 1.0 5.0))
    (Variables|Default|Setpermit%20to%20move true)
    (else
      ;[1 1 1] ... Respawn trigger
      (CallFunction|CheckRespawnHit _returnvalue)
      (if true
        (goto _label)))))

(event EventTick
  (params (DeltaSeconds :type Float%20%28single-precision%29))
  ;[1 1 1] Move the collectable
  (Transformation|AddActorWorldOffset (* (Variables|Default|GetSpeed) (Class|GameplayStatics|GetGlobalTimeDilation))))

(fn ConstructionScript
  (|CallParentFunction))

(fn Spawnkivisound
  ;[1 1 1] spawn sound
  (bind _returnvalue (Audio|SpawnSound2D "/Game/content/Sounds/Explosion02.Explosion02" 1.0 1.0 0.0 0))
  (bind _asitempickp (Utilities|Casting|CastToItempickp (Game|GetGameInstance))))