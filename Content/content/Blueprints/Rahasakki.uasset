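; Money bag pickup that broadcasts its value through the MoneyCollectedED dispatcher when the player overlaps it.
; It recycles itself instead of being destroyed, resetting position and scale, then deriving a new value from the scale result.
; Other overlaps run a respawn-trigger check by object name, but the following branch is fixed true, so they always reset the bag too.
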(event EventBeginPlay
  (|CallParentFunction) ; This node is disabled and will not be called.\nDrag off pins to build functionality.
)

(event Collision|EventActorBeginOverlap
  (params (OtherActor :type Actor%20Object%20Reference))
  (bind _returnvalue (Utilities|GetObjectName OtherActor))
  ;[1 1 1] Check if moneybaag hit...
  (|CallParentFunction OtherActor)
  ;[1 1 1] ... player
  (bind _playercollision (CallFunction|CheckPlayerCollision _returnvalue))
  (if _playercollision
    (Default|CallMoneyCollectedED (Variables|Default|GetValue))
    ;[1 1 1] ... fake moneybag destroy and reset
    (CallFunction|ResetPosition :!label _label)
    (bind _scale (CallFunction|ResetScale))
    (CallFunction|ResetValue _scale)
    (else
      ;[1 1 1] ... Respawn trigger
      (CallFunction|CheckRespawnHit _returnvalue)
      (if true
        (goto _label)))))

(event EventTick
  (params (DeltaSeconds :type Float%20%28single-precision%29))
  (|CallParentFunction DeltaSeconds) ; This node is disabled and will not be called.\nDrag off pins to build functionality.
)

(fn ConstructionScript
  (|CallParentFunction))