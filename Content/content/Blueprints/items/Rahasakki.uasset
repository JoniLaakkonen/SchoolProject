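; Rahasakki is a money bag pickup that is recycled by repositioning instead of being destroyed.
; On player overlap it broadcasts its value through the MoneyCollected event dispatcher and plays a 2D sound, storing the audio component in the Itempickp game instance.
; It then resets position, scale and a scale-derived value.
; Non-player overlaps go through a respawn-trigger check that leads into the same reset.
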(event EventBeginPlay
  (|CallParentFunction) ; This node is disabled and will not be called.\nDrag off pins to build functionality.
)

(event Collision|EventActorBeginOverlap
  (params (OtherActor :type Actor%20Object%20Reference))
  (bind _returnvalue (Utilities|GetObjectName OtherActor))
  ;[1 1 1] Check if moneybaag hit...
  (|CallParentFunction OtherActor)
  ;[1 1 1] ... player
  (bind _playercollision (CallFunction|CheckPlayerCollision _returnvalue))
  (if _playercollision
    (Default|CallMoneyCollectedED (Variables|Default|GetValue))
    (CallFunction|SpawnSound)
    ;[1 1 1] ... fake moneybag destroy and reset
    (CallFunction|ResetPosition :!label _label)
    (bind _scale (CallFunction|ResetScale))
    (CallFunction|ResetValue _scale)
    (else
      ;[1 1 1] ... Respawn trigger
      (CallFunction|CheckRespawnHit _returnvalue)
      (if true
        (goto _label)))))

(event EventTick
  (params (DeltaSeconds :type Float%20%28single-precision%29))
  (|CallParentFunction DeltaSeconds) ; This node is disabled and will not be called.\nDrag off pins to build functionality.
)

(fn ConstructionScript
  (|CallParentFunction))

(fn SpawnSound
  ;[1 1 1] spawn sound
  (bind _returnvalue (Audio|SpawnSound2D "/Game/content/Sounds/mixkit-arcade-retro-game-over-213.mixkit-arcade-retro-game-over-213" 1.0 1.0 0.0 0))
  (bind _asitempickp (Utilities|Casting|CastToItempickp (Game|GetGameInstance)))
  (Variables|/Game/content/Blueprints/Itempickp.Itempickp_C|SetItempickup _asitempickp _returnvalue)
  (Class|GameplayStatics|SetBaseSoundMix "/Game/content/Sounds/Mysoundmix.Mysoundmix"))